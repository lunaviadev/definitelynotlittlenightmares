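; BP_FallingObject is a heavy physics prop that deals lethal-scale damage to an actor it overlaps while flagged as Pushed.
; On BeginPlay its Box and StaticMesh get a large mass scale and start simulating physics.
; A one-shot overlap applies the damage, then destroys the Box after a zero-length delay.
; The first mesh hit from a BP_BullyAI_Static re-enables physics and clears Pushed, which this graph never sets true.
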(event OnComponentHit(StaticMesh)
  (params (HitComponent :type Primitive%20Component%20Object%20Reference) (OtherActor :type Actor%20Object%20Reference) (OtherComp :type Primitive%20Component%20Object%20Reference) (NormalImpulse :type Vector :default "0, 0, 0") (Hit :type Hit%20Result%20Structure%20%28by%20ref%29))
  (Utilities|Casting|CastToBP_BullyAI_Static OtherActor)
  (Utilities|FlowControl|DoOnce false
    (:Completed
      (Physics|SetSimulatePhysics (Variables|Default|GetStaticMesh) true)
      (Variables|Default|SetPushed false))))

(event EventBeginPlay
  (Class|PrimitiveComponent|SetMassScale (Variables|Default|GetBox) "None" 3e+02)
  (Physics|SetSimulatePhysics (Variables|Default|GetBox) true))

(event Collision|EventActorBeginOverlap
  (params (OtherActor :type Actor%20Object%20Reference))
  (bind _output_get (Variables|Default|SetOther%20Actor OtherActor))
  (if (Variables|Default|GetPushed)
    (Utilities|FlowControl|DoOnce false
      (:Completed
        (Game|Damage|ApplyDamage _output_get 9.99e+03 0 0)
        (Utilities|FlowControl|Delay 0.0)
        (Components|DestroyComponent (Variables|Default|GetBox))))))

(fn ConstructionScript)