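; BP_Cube is an interactable box that the third-person character can attach to itself, apparently for pulling.
; Overlaps on its Fwd component toggle a local Pulling flag and the character's CanInteractBox, with debug prints.
; Pressing Q while Pulling attaches the cube to the cached character using KeepRelative rules, and releasing Q detaches it.
; Tick checks the character's interaction flags but leads to an empty sequence.
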(event OnComponentBeginOverlap(Fwd)
  (params (OverlappedComponent :type Primitive%20Component%20Object%20Reference) (OtherActor :type Actor%20Object%20Reference) (OtherComp :type Primitive%20Component%20Object%20Reference) (OtherBodyIndex :type Integer) (bFromSweep :type Boolean) (SweepResult :type Hit%20Result%20Structure%20%28by%20ref%29))
  (Utilities|Casting|CastToBP_ThirdPersonCharacter OtherActor)
  (Variables|Default|SetPulling? true)
  (Development|PrintString "Can Interact" true true "(R=0.193868,G=1.000000,B=0.232411,A=1.000000)" 2.0 "101")
  (Variables|/Game/ThirdPerson/Blueprints/BP_ThirdPersonCharacter.BP_ThirdPersonCharacter_C|SetCanInteractBox? (Variables|Default|GetCharREF) true))

(event OnComponentEndOverlap(Fwd)
  (params (OverlappedComponent :type Primitive%20Component%20Object%20Reference) (OtherActor :type Actor%20Object%20Reference) (OtherComp :type Primitive%20Component%20Object%20Reference) (OtherBodyIndex :type Integer))
  (Utilities|Casting|CastToBP_ThirdPersonCharacter OtherActor)
  (Variables|Default|SetPulling? false)
  (Development|PrintString "Cannot Interact" true true "(R=1.000000,G=0.047707,B=0.000000,A=1.000000)" 2.0 "102")
  (Variables|/Game/ThirdPerson/Blueprints/BP_ThirdPersonCharacter.BP_ThirdPersonCharacter_C|SetCanInteractBox? (Variables|Default|GetCharREF) false))

(event EventBeginPlay
  (bind _returnvalue (Actor|GetActorOfClass "/Game/ThirdPerson/Blueprints/BP_ThirdPersonCharacter.BP_ThirdPersonCharacter_C"))
  (Variables|Default|SetCharREF _returnvalue))

(event Collision|EventActorBeginOverlap
  (params (OtherActor :type Actor%20Object%20Reference)))

(event EventTick
  (params (DeltaSeconds :type Float%20%28single-precision%29))
  (bind _charref (Variables|Default|GetCharREF))
  (if (Variables|/Game/ThirdPerson/Blueprints/BP_ThirdPersonCharacter.BP_ThirdPersonCharacter_C|GetIsInteractingBox? _charref)
    (if (Variables|/Game/ThirdPerson/Blueprints/BP_ThirdPersonCharacter.BP_ThirdPersonCharacter_C|GetCanInteractBox? _charref)
      (Utilities|FlowControl|Sequence))))

(event Input|KeyboardEvents|Q
  (params (Key :type Key%20Structure :default "None"))
  (:Pressed
    (if (Variables|Default|GetPulling?)
      (Transformation|AttachActorToActor (Variables|Default|GetCharREF) "None" "KeepRelative" "KeepRelative" "KeepRelative" true)
      (Development|PrintString "Hello")))
  (:Released
    (Transformation|DetachFromActor "KeepRelative" "KeepRelative" "KeepRelative")
    (Development|PrintString "Hello")))

(fn ConstructionScript)