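; Bully enemy AI character that stands still until pawn sensing fires, then chases the player and attacks.
; On reaching the player via AI MoveTo, it plays a montage, with CanKill gated for the montage's duration.
; Overlap deals light damage, while DealDmage, not called here, applies heavier sphere-overlap damage with debug drawing.
; Incoming damage lowers Health, and Tick destroys the actor below 1.
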(event OnSeePawn(PawnSensing)
  (params (Pawn :type Pawn%20Object%20Reference))
  ;[0.15 0.15 0.15 0.5] Pawn sensing every frame
  (Variables|Default|SetIsSeeingPlayer true)
  (CallFunction|FollowPlayer))

(event Custom|FollowPlayer
  ;[0.15 0.15 0.15 0.5] Ai Move to code
  (Variables|Default|SetCanKill true)
  (if (Variables|Default|GetIsSeeingPlayer)
    (AI|AIMoveTo self "0, 0, 0" (Game|GetPlayerCharacter 0) 7e+01 false
      (:OnSuccess
        (if (Variables|Default|GetCanKill)
          (Variables|Default|SetCanKill false)
          (bind _returnvalue (Animation|PlayAnimMontage 0 1.0 "None"))
          (Utilities|FlowControl|Delay _returnvalue)
          (Variables|Default|SetCanKill true))))
    (else
      (Variables|Default|SetIsSeeingPlayer false))))

(event Custom|Deal%20Dmage
  (bind _attack_sphere (Variables|Default|GetAttack%20Sphere))
  (bind _returnvalue (Transformation|GetWorldLocation _attack_sphere))
  ;[0.15 0.15 0.15 0.5] Deal damage, fixedx
  (bind _outactors (Collision|SphereOverlapActors _returnvalue (Variables|Default|GetSphere%20Radius) (Utilities|Array|MakeArray "ObjectTypeQuery3") "/Game/ThirdPerson/Blueprints/BP_ThirdPersonCharacter.BP_ThirdPersonCharacter_C" (Utilities|Array|MakeArray self)))
  (Rendering|Debug|DrawDebugSphere _returnvalue (Variables|Default|GetSphere%20Radius) 12 "(R=1.000000,G=0.000000,B=0.354175,A=1.000000)" 2.0)
  (for _array_element _outactors
    (Game|Damage|ApplyDamage _array_element 1e+01 (Pawn|GetController) self "/Script/Engine.DamageType")))

(event EventBeginPlay)

(event EventTick
  (params (DeltaSeconds :type Float%20%28single-precision%29))
  ;[0.15 0.15 0.15 0.5] Pawn sensing every frame
  (if (< (Variables|Default|GetHealth) 1.0)
    (Actor|DestroyActor)
    (elif (not (Variables|Default|GetIsSeeingPlayer))
      (Components|Movement|StopMovementImmediately (Variables|Character|GetCharacterMovement)))))

(event Collision|EventActorBeginOverlap
  (params (OtherActor :type Actor%20Object%20Reference))
  ;[0.15 0.15 0.15 0.5] Damages player on overlap with mesh
  (bind _asbp_third_person_character (Utilities|Casting|CastToBP_ThirdPersonCharacter OtherActor))
  (Game|Damage|ApplyDamage _asbp_third_person_character 1.0 0 0))

(event Game|Damage|EventAnyDamage
  (params (Damage :type Float%20%28single-precision%29) (DamageType :type Damage%20Type%20Object%20Reference) (InstigatedBy :type Controller%20Object%20Reference) (DamageCauser :type Actor%20Object%20Reference))
  (Variables|Default|SetHealth (- (Variables|Default|GetHealth) Damage)))

(fn ConstructionScript)