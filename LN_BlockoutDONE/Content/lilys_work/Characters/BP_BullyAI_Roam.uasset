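; BP_BullyAI_Roam is an AI enemy, named as a roaming bully, that detects and damages the third-person player.
; PawnSensing sets the HasSeenPlayer blackboard key on sight, with no logic here to clear it.
; Actor overlap deals light damage to the player.
; The DealDmage event, not called within this graph, applies heavier damage through a sphere overlap at AttackSphere and draws a debug sphere.
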(event OnSeePawn(PawnSensing)
  (params (Pawn :type Pawn%20Object%20Reference))
  ;[0.15 0.15 0.15 0.5] Track player when sensed
  (Utilities|Casting|CastToBP_ThirdPersonCharacter Pawn)
  (AI|Components|Blackboard|SetValueasBool (AI|GetBlackboard (AI|GetAIController self)) (Utilities|Name|MakeLiteralName "HasSeenPlayer") true))

(event Custom|Deal%20Dmage
  (bind _attack_sphere (Variables|Default|GetAttack%20Sphere))
  (bind _returnvalue (Transformation|GetWorldLocation _attack_sphere))
  ;[0.15 0.15 0.15 0.5] Deal damage, fixedx
  (bind _outactors (Collision|SphereOverlapActors _returnvalue (Variables|Default|GetAttack%20Radius) (Utilities|Array|MakeArray "ObjectTypeQuery3") "/Game/ThirdPerson/Blueprints/BP_ThirdPersonCharacter.BP_ThirdPersonCharacter_C" (Utilities|Array|MakeArray self)))
  (Rendering|Debug|DrawDebugSphere _returnvalue (Variables|Default|GetAttack%20Radius) 12 "(R=1.000000,G=0.000000,B=0.354175,A=1.000000)" 2.0)
  (for _array_element _outactors
    (Game|Damage|ApplyDamage _array_element 1e+01 (Pawn|GetController) self "/Script/Engine.DamageType")))

(event EventBeginPlay)

(event EventTick
  (params (DeltaSeconds :type Float%20%28single-precision%29)))

(event Collision|EventActorBeginOverlap
  (params (OtherActor :type Actor%20Object%20Reference))
  ;[0.15 0.15 0.15 0.5] Damages player on overlap with mesh
  (bind _asbp_third_person_character (Utilities|Casting|CastToBP_ThirdPersonCharacter OtherActor))
  (Game|Damage|ApplyDamage _asbp_third_person_character 1.0 0 0))

(fn ConstructionScript)