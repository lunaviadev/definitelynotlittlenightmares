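; BP_Mother is a Red Light, Green Light style watcher that alternately turns away from and toward players, punishing movement.
; Starting on the server, a yaw Timeline plays forward and in reverse, with random pauses between turns.
; While facing players, a looping timer triggers the death event on any player character whose velocity exceeds a small threshold.
; Separately, PawnSensing damages any player character it sees, regardless of movement.
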(event OnSeePawn(PawnSensing)
  (params (Pawn :type Pawn%20Object%20Reference))
  ;[0.15 0.15 0.15 0.5] Damages player if caught in mother's LOS
  (bind _asbp_third_person_character (Utilities|Casting|CastToBP_ThirdPersonCharacter Pawn))
  (Game|Damage|ApplyDamage _asbp_third_person_character 1.0 0 0))

(event Custom|Start%20Look%20Away
  ;[0.15 0.15 0.15 0.5] Rotate mother
  (Variables|Default|SetLookorTurn false)
  (bind _newtrack_0 (Timeline|Timeline PlayFromStart)
    (:Update
      (CallFunction|Rotate (Math|Rotator|MakeRotator 0.0 0.0 _newtrack_0)))
    (:Finished
      (if (Variables|Default|GetLookorTurn)
        (bind _returnvalue (Utilities|Time|SetTimerbyEvent (delegate Custom|Check%20for%20movement) 0.5 true true))
        (Variables|Default|SetCheckPlayerTimer _returnvalue)
        (Utilities|FlowControl|Delay (Math|Random|RandomFloatinRange 1.0 3.5))
        (Utilities|Time|ClearandInvalidateTimerbyHandle (Variables|Default|GetCheckPlayerTimer))
        (CallFunction|StartLookAway)
        (else
          (Utilities|FlowControl|Delay (Math|Random|RandomFloatinRange 1.0 3.5))
          (CallFunction|StartLookPlayer))))))

(event Custom|Start%20Look%20Player
  ;[0.15 0.15 0.15 0.5] Rotate mother
  (Variables|Default|SetLookorTurn true)
  (bind _newtrack_0 (Timeline|Timeline ReverseFromEnd)
    (:Update
      (CallFunction|Rotate (Math|Rotator|MakeRotator 0.0 0.0 _newtrack_0)))
    (:Finished
      (if (Variables|Default|GetLookorTurn)
        (bind _returnvalue (Utilities|Time|SetTimerbyEvent (delegate Custom|Check%20for%20movement) 0.5 true true))
        (Variables|Default|SetCheckPlayerTimer _returnvalue)
        (Utilities|FlowControl|Delay (Math|Random|RandomFloatinRange 1.0 3.5))
        (Utilities|Time|ClearandInvalidateTimerbyHandle (Variables|Default|GetCheckPlayerTimer))
        (CallFunction|StartLookAway)
        (else
          (Utilities|FlowControl|Delay (Math|Random|RandomFloatinRange 1.0 3.5))
          (CallFunction|StartLookPlayer))))))

(event Custom|Rotate
  (params (NewRotation :type Rotator))
  ;[0.15 0.15 0.15 0.5] Rotate mother
  (Transformation|SetWorldRotation (Variables|Character|GetMesh) NewRotation false false))

(event Custom|Check%20for%20movement
  ;[0.15 0.15 0.15 0.5] Rotate mother
  (for _array_element (Variables|/Script/Engine.GameStateBase|GetPlayerArray (Game|GetGameState))
    (bind _asbp_third_person_character (Utilities|Casting|CastToBP_ThirdPersonCharacter (PlayerState|GetPawn _array_element)))
    (if (> (Math|Vector|VectorLength (Transformation|GetVelocity _asbp_third_person_character)) 1e+01)
      (Default|DeathEvent _asbp_third_person_character))))

(event EventBeginPlay
  ;[0.15 0.15 0.15 0.5] Rotate mother
  (Networking|SwitchHasAuthority
    (:Authority
      (Utilities|FlowControl|Delay 3.0)
      (CallFunction|StartLookAway))))

(fn ConstructionScript)